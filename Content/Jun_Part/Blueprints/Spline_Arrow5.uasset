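; Spline_Arrow5 is an arrow actor that travels along the path of the Bp_Spline5 actor found in the level at BeginPlay.
; A Movement timeline, played at a rate set by Speed, drives a Lerp from zero to the spline's length.
; Each update converts that distance to a world-space spline location and applies it through SetActorTransform, without following the spline's rotation.
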(event Custom|Arrow_Move
  (bind _spline_select (Variables|Default|GetSpline_Select))
  (bind _spline (Variables|/Game/Jun_Part/Blueprints/Bp_Spline5.Bp_Spline5_C|GetSpline _spline_select))
  (Components|Timeline|SetPlayRate (Variables|Default|Getmovement) (Variables|Default|GetSpeed))
  (bind _movement (Timeline|movement Play)
    (:Update
      (Transformation|SetActorTransform (Math|Transform|MakeTransform (Spline|GetLocationatDistanceAlongSpline _spline (Math|Float|Lerp 0.0 (Spline|GetSplineLength _spline) _movement) "World") "0, 0, 0" "1.000000,1.000000,1.000000")))))

(event EventBeginPlay
  (bind _returnvalue (Actor|GetActorOfClass "/Game/Jun_Part/Blueprints/Bp_Spline5.Bp_Spline5_C"))
  (Variables|Default|SetSpline_Select _returnvalue)
  (CallFunction|ArrowMove))

(event Collision|EventActorBeginOverlap
  (params (OtherActor :type Actor%20Object%20Reference)))

(event EventTick
  (params (DeltaSeconds :type Float%20%28single-precision%29)))

(fn ConstructionScript)