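; Scene 11 mantle Blueprint that continuously stretches and shrinks a static mesh along the vertical axis.
; BeginPlay caches the mesh's world location and the unscaled height of its bounding box.
; Tick sets Z scale from the absolute sine of game time times MoveZ, keeping X and Y scale.
; It also lowers the mesh by half the scaled height, so a center-pivoted mesh appears to grow downward from its original location.
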(event EventBeginPlay
  (bind _staticmeshcomponent (Variables|Debug|GetStaticMeshComponent))
  (bind _staticmesh (Variables|/Script/Engine.StaticMeshComponent|GetStaticMesh _staticmeshcomponent))
  (bind _returnvalue (StaticMesh|GetBoundingBox _staticmesh))
  (Variables|Default|SetOrigin%20Location (Transformation|GetWorldLocation _staticmeshcomponent))
  (Variables|Default|SetOriginZLength (Math|Float|Absolute(Float) (- (.z (.max _returnvalue)) (.z (.min _returnvalue))))))

(event EventTick
  (params (DeltaSeconds :type Float%20%28single-precision%29))
  (bind _returnvalue (Utilities|Time|GetGameTimeinSeconds))
  (bind _staticmeshcomponent (Variables|Debug|GetStaticMeshComponent))
  (bind _origin_location (Variables|Default|GetOrigin%20Location))
  (bind _move_z (Variables|Default|Getmove_z))
  (bind _returnvalue_2 (Transformation|GetWorldScale _staticmeshcomponent))
  (bind _returnvalue_3 (Math|Trig|Sin(Radians) _returnvalue))
  (bind _returnvalue_4 (* _returnvalue_3 _move_z))
  (bind _returnvalue_5 (Math|Float|Absolute(Float) _returnvalue_4))
  (Transformation|SetWorldScale3D _staticmeshcomponent (Math|Vector|MakeVector (.x _returnvalue_2) (.y _returnvalue_2) _returnvalue_5))
  (Transformation|SetWorldLocation _staticmeshcomponent (Math|Vector|MakeVector (.x _origin_location) (.y _origin_location) (- (.z _origin_location) (* _returnvalue_5 (Variables|Default|GetOriginZLength) 0.5))) false false))

(fn ConstructionScript)