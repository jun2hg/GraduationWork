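; Bp_BlackArrow is an arrow actor for Scene15 that starts in a random orientation and gradually settles to a set angle.
; BeginPlay gives its static mesh a random world rotation on all three axes.
; Tick then eases that rotation with RInterpTo toward a roll equal to the Angle variable, with zero pitch and yaw.
; The file never assigns Angle.
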(event EventBeginPlay
  (Transformation|SetWorldRotation (Variables|Debug|GetStaticMeshComponent) (Math|Rotator|MakeRotator (Math|Random|RandomFloatinRange 3.6e+02 -3.6e+02) (Math|Random|RandomFloatinRange 3.6e+02 -3.6e+02) (Math|Random|RandomFloatinRange 3.6e+02 -3.6e+02)) false false))

(event Collision|EventActorBeginOverlap
  (params (OtherActor :type Actor%20Object%20Reference)))

(event EventTick
  (params (DeltaSeconds :type Float%20%28single-precision%29))
  (bind _staticmeshcomponent (Variables|Debug|GetStaticMeshComponent))
  (Transformation|SetWorldRotation _staticmeshcomponent (Math|Interpolation|RInterpTo (Transformation|GetWorldRotation _staticmeshcomponent) (Math|Rotator|MakeRotator (Variables|Default|GetAngle) 0.0 0.0) DeltaSeconds 1.0) false false))

(fn ConstructionScript)