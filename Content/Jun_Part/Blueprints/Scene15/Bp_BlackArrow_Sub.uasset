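; Scene 15 black arrow actor that spins its static mesh from a random orientation, then turns it toward a set pitch.
; On BeginPlay it picks a random origin rotation, and a timeline lerps the mesh's roll and yaw a quarter turn either side of it.
; Tick waits on a delay of several seconds, then eases the mesh toward the Angle pitch with quaternion slerp scaled by delta time.
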(event EventBeginPlay
  (bind _returnvalue (Math|Random|RandomFloatinRange 3.6e+02 -3.6e+02))
  (bind _returnvalue_2 (Math|Random|RandomFloatinRange 3.6e+02 -3.6e+02))
  (bind _returnvalue_3 (Math|Random|RandomFloatinRange 3.6e+02 -3.6e+02))
  (bind _returnvalue_4 (Math|Rotator|MakeRotator _returnvalue_2 _returnvalue_3 _returnvalue))
  (Transformation|SetWorldRotation (Variables|Debug|GetStaticMeshComponent) _returnvalue_4 false false)
  (Variables|Default|SetOriginRotator _returnvalue_4)
  (bind _alpha (Timeline|타임라인 Play)
    (:Update
      (Transformation|SetWorldRotation (Variables|Debug|GetStaticMeshComponent) (Math|Rotator|Lerp(Rotator) (Math|Rotator|MakeRotator (- (.roll (Variables|Default|GetOriginRotator)) 9e+01) (.pitch (Variables|Default|GetOriginRotator)) (- (.yaw (Variables|Default|GetOriginRotator)) 9e+01)) (Math|Rotator|MakeRotator (+ (.roll (Variables|Default|GetOriginRotator)) 9e+01) (.pitch (Variables|Default|GetOriginRotator)) (+ (.yaw (Variables|Default|GetOriginRotator)) 9e+01)) _alpha) false false))))

(event Collision|EventActorBeginOverlap
  (params (OtherActor :type Actor%20Object%20Reference)))

(event EventTick
  (params (DeltaSeconds :type Float%20%28single-precision%29))
  (bind _staticmeshcomponent (Variables|Debug|GetStaticMeshComponent))
  ;[1 1 1] 정지 후 방향 전환
  (if (Variables|Default|GetIsStart)
    (Transformation|SetWorldRotation _staticmeshcomponent (Class|KismetMathLibrary|QuatRotator (Class|KismetMathLibrary|QuatSlerp (Math|Conversions|ToQuaternion(Rotator) (Transformation|GetWorldRotation _staticmeshcomponent)) (Math|Conversions|ToQuaternion(Rotator) (Math|Rotator|MakeRotator 0.0 (Variables|Default|GetAngle) 0.0)) (* DeltaSeconds 1.0))) false false)
    (else
      (Utilities|FlowControl|Delay 7.5)
      (Variables|Default|SetIsStart true))))

(fn ConstructionScript)