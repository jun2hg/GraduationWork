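; Black arrow actor for Scene15 whose mesh starts at a random orientation and later eases toward a target angle.
; BeginPlay randomizes the mesh's world rotation, and Tick waits 7.5 seconds through a Delay before setting IsStart.
; Tick then quaternion-slerps the mesh each frame toward a pitch of Angle, with zero roll and yaw.
; TickEventStop clears a TickActive flag, which Tick does not read.
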(event EventBeginPlay
  (Transformation|SetWorldRotation (Variables|Debug|GetStaticMeshComponent) (Math|Rotator|MakeRotator (Math|Random|RandomFloatinRange 3.6e+02 -3.6e+02) (Math|Random|RandomFloatinRange 3.6e+02 -3.6e+02) (Math|Random|RandomFloatinRange 3.6e+02 -3.6e+02)) false false))

(event Collision|EventActorBeginOverlap
  (params (OtherActor :type Actor%20Object%20Reference)))

(event EventTick
  (params (DeltaSeconds :type Float%20%28single-precision%29))
  (bind _staticmeshcomponent (Variables|Debug|GetStaticMeshComponent))
  ;[1 1 1] 정지 후 방향 전환
  (if (Variables|Default|GetIsStart)
    (Transformation|SetWorldRotation _staticmeshcomponent (Class|KismetMathLibrary|QuatRotator (Class|KismetMathLibrary|QuatSlerp (Math|Conversions|ToQuaternion(Rotator) (Transformation|GetWorldRotation _staticmeshcomponent)) (Math|Conversions|ToQuaternion(Rotator) (Math|Rotator|MakeRotator 0.0 (Variables|Default|GetAngle) 0.0)) (* DeltaSeconds 1.0))) false false)
    (else
      (Utilities|FlowControl|Delay 7.5)
      (Variables|Default|SetIsStart true))))

(fn ConstructionScript)

(fn TickEventStop
  (Variables|Default|SetTick_Active false))