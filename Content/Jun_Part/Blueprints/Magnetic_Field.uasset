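; Magnetic field actor that aims to build an animated dynamic mesh along a spline; the generation logic is unfinished.
; Tick accumulates time and passes it to UpdateMesh, which derives a point count and even spacing from spline length and target point distance.
; It then caches the dynamic mesh and clears the transform array, but the per-point loop is empty and the time-based offset math is unconnected.
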(event EventBeginPlay)

(event Collision|EventActorBeginOverlap
  (params (OtherActor :type Actor%20Object%20Reference)))

(event EventTick
  (params (DeltaSeconds :type Float%20%28single-precision%29))
  (bind _output_get (Variables|Default|Setaccum_time (+ DeltaSeconds (Variables|Default|Getaccum_time))))
  (CallFunction|UpdateMesh _output_get))

(fn ConstructionScript)

(fn UpdateMesh
  (params (Time :type Float%20%28double-precision%29))
  (bind _spline (Variables|Default|GetSpline))
  (bind _returnvalue (Spline|GetSplineLength _spline))
  (Variables|Default|SetTNormalized (Math|Float|%(Float) Time (* Time (Variables|Default|GetSpeed))))
  (bind _output_get (Variables|Default|SetSplinePoints (+ (.ReturnValue (Math|Float|Division(WholeandRemainder) _returnvalue (Math|Conversions|ToFloat(Integer) (Variables|Default|GetPoints%20Dist)))) 1)))
  (Variables|Default|SetNew%20Points%20Dist (/ _returnvalue (- _output_get 1)))
  (Utilities|FlowControl|Sequence
    (:then_0
      (bind _returnvalue_2 (DynamicMeshComponent|GetDynamicMesh (Variables|DynamicMeshActor|GetDynamicMeshComponent)))
      (Variables|Default|SetDynVar _returnvalue_2)
      (Utilities|Array|Clear (Variables|Default|GetTransforms))
      (for _index (range 0 (Variables|Default|GetSplinePoints))
        _))))