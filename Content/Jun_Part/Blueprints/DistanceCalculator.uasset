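; DistanceCalculator logs how closely the VR player's view lines up with the actors they look at.
; A one-second looping timer traces from the pawn root along the VR camera's forward vector and maps impact-to-actor-center distance to an inverse score.
; Nonzero scores count as hits, and each sample is appended to a result string.
; EndPlay saves that string and the total hit time to a text file.
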(event EventBeginPlay
  (Utilities|Time|SetTimerbyFunctionName 0 "CalculateAndSaveDists" 1.0 true))

(event EventEndPlay
  (params (EndPlayReason :type EEndPlayReason%20Enum :default "Destroyed"))
  ;[1 1 1] Save File
  (Class|BPFLSaveFile|SaveTexttoFile (Utilities|String|Append (Variables|Default|GetResult) (Utilities|String|Append (Utilities|String|ToString(Integer) (Variables|Default|GetTotal_Hit_Time)) " 
")) "test.txt"))

(fn ConstructionScript)

(fn CalculateandSaveDists
  (bind _returnvalue (Game|GetPlayerController 0))
  (bind _returnvalue_2 (Pawn|GetControlledPawn _returnvalue))
  (bind _rootcomponent (Variables|/Script/Engine.Actor|GetRootComponent _returnvalue_2))
  (bind _returnvalue_3 (Transformation|GetWorldLocation _rootcomponent))
  (bind _aspc_vr (Utilities|Casting|CastToPC_VR _returnvalue))
  (bind _outhit (Collision|LineTraceByChannel _returnvalue_3 (+ _returnvalue_3 (* (Math|Vector|GetForwardVector (Transformation|GetWorldRotation (Variables|/Game/Blueprint/PC_VR.PC_VR_C|GetVR_Camera _aspc_vr))) 1.5e+03)) "TraceTypeQuery1" false 0 "ForOneFrame"))
  (Variables|Default|SetNormalized_Dist (Math|Float|Lerp 1e+03 0.0 (Math|Float|Clamp(Float) (/ (Math|Vector|Distance(Vector) (.ImpactPoint (Collision|BreakHitResult _outhit)) (Transformation|GetActorLocation (.HitActor (Collision|BreakHitResult _outhit)))) 4e+02))))
  ;[1 1 1] Hit num
  (if (!= (Variables|Default|GetNormalized_Dist) 0.0)
    (Variables|Default|SetOn_Hit "O")
    (Variables|Default|SetTotal_On_Hit (+ (Variables|Default|GetTotal_On_Hit) 1))
    ;[1 1 1] Hit time
    (Variables|Default|SetHit_Time "1")
    (Variables|Default|SetTotal_Hit_Time (+ (Variables|Default|GetTotal_Hit_Time) 1))
    (else
      (Variables|Default|SetOn_Hit "X")
      (Variables|Default|SetHit_Time "0")))
  (Variables|Default|SetResult (Utilities|String|Append (Variables|Default|GetResult) (Utilities|String|Append (Utilities|String|Append (Utilities|String|Append (Utilities|String|Append (Utilities|String|ToString(Float) (Variables|Default|GetNormalized_Dist)) "  ") (Utilities|String|Append (Variables|Default|GetOn_Hit) "  ")) (Utilities|String|Append (Variables|Default|GetHit_Time) "  ")) " 
"))))