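; Bp_Cube is an actor that moves continuously along a circular path in the world Y-Z plane.
; Each Tick adds delta seconds to an accumulated Time, then sets the actor's world location from cosine and sine of Time, scaled by three times Radius.
; The location is absolute rather than relative to the placed position, and BeginPlay, overlap and construction logic are empty.
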(event EventBeginPlay)

(event Collision|EventActorBeginOverlap
  (params (OtherActor :type Actor%20Object%20Reference)))

(event EventTick
  (params (DeltaSeconds :type Float%20%28single-precision%29))
  (bind _radius (Variables|Default|GetRadius))
  (bind _output_get (Variables|Default|SetTime (+ DeltaSeconds (Variables|Default|GetTime))))
  (Transformation|SetActorLocation (Math|Vector|MakeVector 0.0 (* (* (Math|Trig|Cos(Radians) _output_get) _radius) 3.0) (* (* (Math|Trig|Sin(Radians) _output_get) _radius) 3.0)) false false))

(fn ConstructionScript)