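; Magnetic field actor that shows arrowheads flowing along a spline, built with Geometry Script on a dynamic mesh.
; MagneticActivate plays a timeline that drives UpdateMesh, or stops it and hides the actor; activating does not unhide it.
; Each update resets the mesh and appends ArrowHead copies at evenly fitted spacing, Z aligned to the tangent.
; Wrapping time scaled by Speed shifts them one spacing per cycle for seamless looping motion.
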(event Custom|Magnetic%20Activate
  (params (Switch :type Boolean))
  (if Switch
    (bind _time (Timeline|타임라인 Play)
      (:Update
        (CallFunction|UpdateMesh _time false)))
    (else
      (Utilities|FlowControl|Sequence
        (:then_0
          (Timeline|타임라인 Stop))
        (:then_1
          (Rendering|SetActorHiddenInGame true))))))

(event EventBeginPlay)

(event Collision|EventActorBeginOverlap
  (params (OtherActor :type Actor%20Object%20Reference)))

(event EventTick
  (params (DeltaSeconds :type Float%20%28single-precision%29)))

(fn ConstructionScript)

(fn UpdateMesh
  (params (Time :type Float%20%28double-precision%29) (NewParam :type Boolean))
  (bind _spline (Variables|Default|GetSpline))
  (bind _spline_2 (Variables|Default|GetSpline))
  (bind _returnvalue (Spline|GetSplineLength _spline_2))
  ;[1 1 1] Set Up
  (Variables|Default|SetTNormalized (Math|Float|%(Float) (* Time (Variables|Default|GetSpeed)) 1.0))
  (bind _output_get (Variables|Default|SetSplinePoints (+ (.ReturnValue (Math|Float|Division(WholeandRemainder) _returnvalue (Math|Conversions|ToFloat(Integer) (Variables|Default|GetPoints%20Dist)))) 1)))
  (Variables|Default|SetNew%20Points%20Dist (/ _returnvalue (- _output_get 1)))
  (Utilities|FlowControl|Sequence
    (:then_0
      ;[1 1 1] Generate Spline Points
      (bind _returnvalue_2 (DynamicMeshComponent|GetDynamicMesh (Variables|DynamicMeshActor|GetDynamicMeshComponent)))
      (bind _output_get_2 (Variables|Default|SetDynVar _returnvalue_2))
      (DynamicMesh|Reset _output_get_2)
      (Utilities|Array|Clear (Variables|Default|GetTransforms))
      (for _index (range 0 (Variables|Default|GetSplinePoints))
        (Utilities|Array|Add (Variables|Default|GetTransforms) (Math|Transform|MakeTransform (.location (Spline|GetTransformatDistanceAlongSpline _spline (Math|Float|%(Float) (+ (* (Variables|Default|GetTNormalized) (Variables|Default|GetNew%20Points%20Dist)) (* _index (Variables|Default|GetNew%20Points%20Dist))) (Spline|GetSplineLength (Variables|Default|GetSpline))) "Local" false)) (Math|Rotator|MakeRotfromZ (Spline|GetTangentatDistanceAlongSpline _spline (Math|Float|%(Float) (+ (* (Variables|Default|GetTNormalized) (Variables|Default|GetNew%20Points%20Dist)) (* _index (Variables|Default|GetNew%20Points%20Dist))) (Spline|GetSplineLength (Variables|Default|GetSpline))) "Local")) (.scale (Spline|GetTransformatDistanceAlongSpline _spline (Math|Float|%(Float) (+ (* (Variables|Default|GetTNormalized) (Variables|Default|GetNew%20Points%20Dist)) (* _index (Variables|Default|GetNew%20Points%20Dist))) (Spline|GetSplineLength (Variables|Default|GetSpline))) "Local" false))))))
    (:then_1
      (bind _arrowhead (Variables|Default|GetArrowHead)
        (:then
          (bind _returnvalue_3 (DynamicMeshActor|AllocateComputeMesh))
          (bind _returnvalue_4 (GeometryScript|StaticMesh|CopyMeshFromStaticMesh :FromStaticMeshAsset _arrowhead :ToDynamicMesh _returnvalue_3 :Debug 0)
            (:Success
              (Class|GeometryScriptLibraryMeshBasicEditFunctions|AppendMeshTransformed :TargetMesh (Variables|Default|GetDynVar) :AppendMesh _returnvalue_4 :AppendTransforms (Variables|Default|GetTransforms) :AppendOptions "(CombineMode=EnableAllMatching)" :Debug 0))))
        (:else)))))